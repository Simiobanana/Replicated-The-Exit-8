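; Security camera actor that switches between a normal fixed pose and an anomaly state in which it turns to track the player.
; The anomaly event re-arms a fast looping timer on itself, yawing the camera mesh toward the player controller's focal location with a quarter-turn offset.
; The normal event clears that timer and, after a short delay, snaps the mesh back to its fixed rotation.
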(event `self.ReceiveTick`
  (params (DeltaSeconds :type "Float (single-precision)")))

(event `Camera normal`
  ;[1 0.807 0.1156] Normal
  (`KismetSystemLibrary.K2_ClearAndInvalidateTimerHandle` (`self.CameraTimer`))
  (`KismetSystemLibrary.Delay` 0.2)
  (`SceneComponent.K2_SetWorldRotation` (`self.SecurityCamera_Cube_001`) (`KismetMathLibrary.MakeRotator` 0.0 0.0 -90.0) false false))

(event `Camera anomaly`
  (bind (_returnvalue_roll _returnvalue_pitch _returnvalue_yaw) (`KismetMathLibrary.BreakRotator` (`KismetMathLibrary.FindLookAtRotation` (`SceneComponent.K2_GetComponentLocation` (`self.SecurityCamera_Cube_001`)) (`PlayerController.GetFocalLocation` (`GameplayStatics.GetPlayerController` 0)))))
  ;[1 0.4048 0.4446] Anomalia
  (bind _returnvalue (`KismetSystemLibrary.K2_SetTimerDelegate` (delegate `Camera anomaly`) 0.01 true))
  (set `self.CameraTimer` _returnvalue)
  (`SceneComponent.K2_SetWorldRotation` (`self.SecurityCamera_Cube_001`) (`KismetMathLibrary.MakeRotator` 0.0 0.0 (+ _returnvalue_yaw 90.0)) false false))

(fn `UserConstructionScript`)