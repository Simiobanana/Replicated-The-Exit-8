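; Teleport trigger for an anomaly-spotting loop: its box overlap advances or resets level progress based on TieneAnomalias.
; If true, it increments the Cartel sign's counter, moves the player to DestinationFanomaly, resets the spline NPC and calls Anomalias on Modular_Zone.
; Otherwise it zeroes the counter and moves the player to Destination, keeping their rotation.
; The sign updates before the player cast; the level-eight check and Endgame are empty.
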(event `self.Box.OnComponentBeginOverlap`
  (params (OverlappedComponent :type "PrimitiveComponent Object Reference") (OtherActor :type "Actor Object Reference") (OtherComp :type "PrimitiveComponent Object Reference") (OtherBodyIndex :type Integer) (bFromSweep :type Boolean) (SweepResult :type "HitResult Structure (by ref)"))
  (bind _destinationfanomaly (`self.DestinationFanomaly`))
  (bind _returnvalue (`SceneComponent.K2_GetComponentRotation` _destinationfanomaly))
  ;[1 1 1] LevelSign
  (if (`self.Tiene anomalias`)
    (`KismetSystemLibrary.PrintString` "NextLvl")
    (bind _output (`|GetArrayItem` (stale `self.ReceiveBeginPlay` _outactors)))
    (`/Game/Blueprints/Cartel.LevelChange` _output)
    (bind _output_get (set `/Game/Blueprints/Cartel.NivelCambio` (+ (`/Game/Blueprints/Cartel.NivelCambio` _output) 1) _output))
    (bind _asbp_first_person_character (cast `/Game/FirstPerson/Blueprints/BP_FirstPersonCharacter` OtherActor))
    (`self.K2_SetActorLocationAndRotation` _asbp_first_person_character (`SceneComponent.K2_GetComponentLocation` _destinationfanomaly) _returnvalue false false)
    (`self.K2_SetActorRotation` _asbp_first_person_character _returnvalue false)
    (bind _outactors (`GameplayStatics.GetAllActorsOfClass` "/Game/AI/AI_Characters/Spline/BP_SplineNPC.BP_SplineNPC_C"))
    (`/Game/AI/AI_Characters/Spline/BP_SplineNPC.ResetSplinePos` (`|GetArrayItem` _outactors))
    (bind _outactors_2 (`GameplayStatics.GetAllActorsOfClass` "/Game/Blueprints/Modular_Zone.Modular_Zone_C"))
    (`/Game/Blueprints/Modular_Zone.Anomalias` (`|GetArrayItem` _outactors_2))
    (if (>= _output_get 8)
      _)
    (else
      (`KismetSystemLibrary.PrintString` "Reset")
      (`/Game/Blueprints/Cartel.LevelReset` _output)
      (set `/Game/Blueprints/Cartel.NivelCambio` 0 _output)
      ;[1 0.08854 0.08854] xd
      (bind _asbp_first_person_character_2 (cast `/Game/FirstPerson/Blueprints/BP_FirstPersonCharacter` OtherActor))
      (`self.K2_SetActorLocationAndRotation` _asbp_first_person_character_2 (`SceneComponent.K2_GetComponentLocation` (`self.Destination`)) (`SceneComponent.K2_GetComponentRotation` (`Actor.RootComponent` _asbp_first_person_character_2)) false false))))

(event `self.ReceiveBeginPlay`
  (bind _outactors (`GameplayStatics.GetAllActorsOfClass` "/Game/Blueprints/Cartel.Cartel_C")))

(fn `UserConstructionScript`)