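; Ceiling lamp actor that switches between normal lighting and an anomalous flicker.
; LucesAnomalia re-triggers itself on a 0.1-second timer, using a resetting DoOnce and random delay to toggle the RectLight and alternate lit and unlit lamp materials via FlipFlop.
; LucesNormales clears that timer and restores the lit state after a short delay.
; ResetLevel briefly switches the RectLight off, then back on.
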(event `ResetLevel`
  (`SceneComponent.SetVisibility` (`self.RectLight`) false true)
  (`KismetSystemLibrary.Delay` 0.5)
  (`SceneComponent.SetVisibility` (`self.RectLight`) true true))

(event `self.ReceiveTick`
  (params (DeltaSeconds :type "Float (single-precision)")))

(event `LucesNormales`
  (`KismetSystemLibrary.K2_ClearAndInvalidateTimerHandle` (`self.Timer`))
  (`KismetSystemLibrary.Delay` 0.3)
  (`PrimitiveComponent.SetMaterial` (`self.CeilingLamp_Baked`) 0 "/Game/Models/CeilingLights/Baked.Baked")
  (`SceneComponent.SetVisibility` (`self.RectLight`) true true))

(event `LucesAnomalia`
  (bind _returnvalue (`KismetSystemLibrary.K2_SetTimerDelegate` (delegate `LucesAnomalia`) 0.1 true))
  (set `self.Timer` _returnvalue)
  (`/Engine/EditorBlueprintResources/StandardMacros.DoOnce` false :!label _label
    (:`Completed`
      (`KismetSystemLibrary.RetriggerableDelay` (`KismetMathLibrary.RandomFloatInRange` 0.1 0.6))
      (`SceneComponent.ToggleVisibility` (`self.RectLight`) false)
      (`/Engine/EditorBlueprintResources/StandardMacros.FlipFlop`
        (:`A`
          (`PrimitiveComponent.SetMaterial` (`self.CeilingLamp_Baked`) 0 "/Game/Models/CeilingLights/Baked.Baked")
          (goto _label :!via `Reset`))
        (:`B`
          (`PrimitiveComponent.SetMaterial` (`self.CeilingLamp_Baked`) 0 "/Game/Models/CeilingLights/BakedOff.BakedOff")
          (goto _label :!via `Reset`))))))

(fn `UserConstructionScript`)