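; Cartel is a sign Blueprint that displays the current level number through a text render component.
; On BeginPlay it writes the NivelCambio counter to TextRender1 and uniformly shrinks the Station2Plane018 component.
; LevelChange increments the counter and LevelReset sets it back to zero, each then refreshing the displayed text.
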(event `self.ReceiveBeginPlay`
  (`TextRenderComponent.K2_SetText` (`self.TextRender1`) (`KismetTextLibrary.Conv_IntToText` (`self.NivelCambio`)))
  (`SceneComponent.SetWorldScale3D` (`self.station2_Plane_018`) (0.35 0.35 0.35)))

(event `LevelReset`
  (bind _textrender1 (`self.TextRender1`))
  ;[1 0.3978 0] Reiniciar texto de nivel
  (bind _output_get (set `self.NivelCambio` 0))
  (`TextRenderComponent.K2_SetText` _textrender1 (`KismetTextLibrary.Conv_IntToText` _output_get))
  (set `self.TextRender1` _textrender1))

(event `LevelChange`
  (bind _textrender1 (`self.TextRender1`))
  ;[1 0.9023 0] Texto del nivel actual
  (bind _output_get (set `self.NivelCambio` (+ (`self.NivelCambio`) 1)))
  (`TextRenderComponent.K2_SetText` _textrender1 (`KismetTextLibrary.Conv_IntToText` _output_get))
  (set `self.TextRender1` _textrender1))

(fn `UserConstructionScript`)