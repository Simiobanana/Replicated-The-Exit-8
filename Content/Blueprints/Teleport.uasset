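; Teleport trigger for a looping anomaly level: moves the first-person player to a Destination, keeping rotation, and resets spline NPCs and ceiling lights.
; If TieneAnomalias is set, it resets the level sign (Cartel) and its NivelCambio counter; otherwise it advances both.
; It then calls Anomalias on the first Modular_Zone.
; Separate Enabled and Disabled overlap volumes toggle the teleport box's collision.
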(event `self.ReceiveBeginPlay`
  (bind _outactors (`GameplayStatics.GetAllActorsOfClass` "/Game/Blueprints/Cartel.Cartel_C")))

(event `self.Box.OnComponentBeginOverlap`
  (params (OverlappedComponent :type "PrimitiveComponent Object Reference") (OtherActor :type "Actor Object Reference") (OtherComp :type "PrimitiveComponent Object Reference") (OtherBodyIndex :type Integer) (bFromSweep :type Boolean) (SweepResult :type "HitResult Structure (by ref)"))
  (bind _asbp_first_person_character (cast `/Game/FirstPerson/Blueprints/BP_FirstPersonCharacter` OtherActor))
  (`self.K2_SetActorLocationAndRotation` _asbp_first_person_character (`SceneComponent.K2_GetComponentLocation` (`self.Destination`)) (`SceneComponent.K2_GetComponentRotation` (`Actor.RootComponent` _asbp_first_person_character)) false false)
  (bind _outactors (`GameplayStatics.GetAllActorsOfClass` "/Game/AI/AI_Characters/Spline/BP_SplineNPC.BP_SplineNPC_C"))
  (`/Game/AI/AI_Characters/Spline/BP_SplineNPC.ResetSplinePos` _outactors)
  (bind _outactors_2 (`GameplayStatics.GetAllActorsOfClass` "/Game/Blueprints/CeilingLights.CeilingLights_C"))
  (`/Game/Blueprints/CeilingLights.ResetLevel` _outactors_2)
  (if (`self.TieneAnomalias`)
    (`KismetSystemLibrary.PrintString` "Reset")
    (bind _output (`|GetArrayItem` (stale `self.ReceiveBeginPlay` _outactors)))
    (`/Game/Blueprints/Cartel.LevelReset` _output)
    (bind _output_get (set `/Game/Blueprints/Cartel.NivelCambio` 0 _output))
    (`KismetSystemLibrary.PrintString` (`KismetStringLibrary.Conv_IntToString` _output_get))
    (else
      (`KismetSystemLibrary.PrintString` "SiguienteNivel")
      (`/Game/Blueprints/Cartel.LevelChange` _output)
      (bind _output_get_2 (set `/Game/Blueprints/Cartel.NivelCambio` (+ (`/Game/Blueprints/Cartel.NivelCambio` _output) 1) _output))
      (`KismetSystemLibrary.PrintString` (`KismetStringLibrary.Conv_IntToString` _output_get_2))))
  (bind _outactors_3 (`GameplayStatics.GetAllActorsOfClass` "/Game/Blueprints/Modular_Zone.Modular_Zone_C"))
  (`/Game/Blueprints/Modular_Zone.Anomalias` (`|GetArrayItem` _outactors_3)))

(event `self.Enabled.OnComponentBeginOverlap`
  (params (OverlappedComponent :type "PrimitiveComponent Object Reference") (OtherActor :type "Actor Object Reference") (OtherComp :type "PrimitiveComponent Object Reference") (OtherBodyIndex :type Integer) (bFromSweep :type Boolean) (SweepResult :type "HitResult Structure (by ref)"))
  ;[1 0 0.7219] Desactivar/ActivarTP
  (cast `/Game/FirstPerson/Blueprints/BP_FirstPersonCharacter` OtherActor)
  (`KismetSystemLibrary.PrintString` "Activado")
  (`PrimitiveComponent.SetCollisionEnabled` (`self.Box`) "QueryAndPhysics"))

(event `self.Disabled.OnComponentBeginOverlap`
  (params (OverlappedComponent :type "PrimitiveComponent Object Reference") (OtherActor :type "Actor Object Reference") (OtherComp :type "PrimitiveComponent Object Reference") (OtherBodyIndex :type Integer) (bFromSweep :type Boolean) (SweepResult :type "HitResult Structure (by ref)"))
  ;[1 0 0.7219] Desactivar/ActivarTP
  (cast `/Game/FirstPerson/Blueprints/BP_FirstPersonCharacter` OtherActor)
  (`KismetSystemLibrary.PrintString` "desactivado")
  (`PrimitiveComponent.SetCollisionEnabled` (`self.Box`) "NoCollision"))

(fn `UserConstructionScript`)